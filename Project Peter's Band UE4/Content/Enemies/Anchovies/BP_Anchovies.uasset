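; BP_Anchovies is an enemy pawn that patrols an array of TargetPoints in a loop.
; Each step checks for a nav path, uses AI MoveTo, then advances on success or failure.
; Overlapping a "Light"-tagged actor path-checks the farther of the previous and current points, despite the helper's name ReturnShorterDistance.
; An invalid path advances the patrol, while the retreat move is disconnected and never runs.
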(event `self.ReceiveBeginPlay`
  (set `self.Point Iterator` -1)
  (bind _returnvalue (`AddComponent|StaticMeshComponent_12` :`RelativeTransform` (`KismetMathLibrary.MakeTransform` (0.0 0.0 0.0))))
  (`StaticMeshComponent.SetStaticMesh` _returnvalue null)
  (`self.Patrol To Next`))

(event `Patrol To Next`
  (bind _output_get (set `self.Point Iterator` (+ (`self.Point Iterator`) 1)))
  (bind _returnvalue (`self.K2_GetActorLocation` (`KismetArrayLibrary.Array_Get` (`self.Target Points`) _output_get)))
  (bind _returnvalue_2 (`NavigationSystem.FindPathToLocationSynchronously` (`self.K2_GetActorLocation`) _returnvalue))
  (if (`KismetSystemLibrary.IsValid` _returnvalue_2)
    (`|AIMoveTo` self _returnvalue null 5.0 true
      (:`then`
        (if (== _output_get (- (`KismetArrayLibrary.Array_Length` (`self.Target Points`)) 1))
          (set `self.Point Iterator` -1)))
      (:`OnSuccess`
        (`self.Patrol To Next` :!label _label))
      (:`OnFail`
        (goto _label)))
    (else
      (goto _label))))

(event `self.ReceiveActorBeginOverlap`
  (params (OtherActor :type "Actor Object Reference"))
  (if (`self.ActorHasTag` OtherActor "Light")
    (bind _newparam2 (`self.Return shorter distance` (`KismetArrayLibrary.Array_Get` (`self.Target Points`) (+ (stale `Patrol To Next` _output_get) -1)) (`KismetArrayLibrary.Array_Get` (`self.Target Points`) (stale `Patrol To Next` _output_get))))
    (bind _returnvalue (`NavigationSystem.FindPathToLocationSynchronously` (`self.K2_GetActorLocation`) _newparam2))
    (if (not (`KismetSystemLibrary.IsValid` _returnvalue))
      (goto _label))))

(fn `Return shorter distance`
  (params (NewParam :type "Actor Object Reference") (NewParam1 :type "Actor Object Reference"))
  (returns (NewParam2 :type "Vector Structure"))
  (`/Engine/EditorBlueprintResources/StandardMacros.CompareFloat` (`self.GetDistanceTo` NewParam) (`self.GetDistanceTo` NewParam1)
    (:`>`
      (return (`self.K2_GetActorLocation` NewParam)))
    (:`==`
      _)
    (:`<`
      _))
  (return (`self.K2_GetActorLocation` NewParam1)))

(fn `UserConstructionScript`)