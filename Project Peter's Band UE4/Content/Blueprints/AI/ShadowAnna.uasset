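; ShadowAnna is an AI character that moves along TargetPoints, advancing when a Player-tagged actor overlaps it or OnMessgae fires.
; Each advance increments PointIterator and, if a synchronous path query returns a valid object, issues AIMoveTo to that point.
; Tick sets walk speed from player distance within a clamped range, so it speeds up as the player nears.
; The ReturnShorterDistance helper is never called here.
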(event `self.ReceiveTick`
  (params (DeltaSeconds :type "Float (single-precision)"))
  (bind _returnvalue (- 1500.0 (* (`self.GetDistanceTo` (`GameplayStatics.GetPlayerCharacter` 0)) 1.5)))
  (bind _returnvalue_2 (`KismetMathLibrary.SelectFloat` 700.0 _returnvalue (> _returnvalue 700.0)))
  (set `CharacterMovementComponent.MaxWalkSpeed` (`KismetMathLibrary.SelectFloat` 100.0 _returnvalue_2 (< _returnvalue_2 100.0)) (`self.CharacterMovement`)))

(event `OnMessgae`
  (bind _output_get (set `self.Point Iterator` (+ (`self.Point Iterator`) 1) :!label _label))
  (bind _returnvalue (`self.K2_GetActorLocation` (`KismetArrayLibrary.Array_Get` (`self.Target Points`) _output_get)))
  (bind _returnvalue_2 (`NavigationSystem.FindPathToLocationSynchronously` (`self.K2_GetActorLocation`) _returnvalue))
  (if (`KismetSystemLibrary.IsValid` _returnvalue_2)
    (`|AIMoveTo` "0" self _returnvalue null 5.0 true
      (:`then`
        (if (== _output_get 0)
          (set `self.Point Iterator` -1))))))

(event `self.ReceiveActorBeginOverlap`
  (params (OtherActor :type "Actor Object Reference"))
  (if (`self.ActorHasTag` OtherActor "Player")
    (goto _label)))

(fn `Return shorter distance`
  (params (NewParam :type "Actor Object Reference") (NewParam1 :type "Actor Object Reference"))
  (returns (NewParam2 :type "Vector Structure"))
  (`/Engine/EditorBlueprintResources/StandardMacros.CompareFloat` (`self.GetDistanceTo` NewParam) (`self.GetDistanceTo` NewParam1 null)
    (:`>`
      (return (`self.K2_GetActorLocation` NewParam)))
    (:`==`
      _)
    (:`<`
      _))
  (return (`self.K2_GetActorLocation` NewParam1)))

(fn `UserConstructionScript`)