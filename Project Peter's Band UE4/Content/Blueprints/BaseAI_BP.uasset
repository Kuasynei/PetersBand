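; Base AI pawn that patrols endlessly through an array of target points.
; On BeginPlay it adds a sphere static mesh component and starts moving to the first point.
; PatrolToNext advances an index and calls AIMoveTo on that point's location, resetting the index after the last point so the route loops.
; Both success and failure of a move trigger the next leg, so an unreachable point is skipped.
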(event `self.ReceiveBeginPlay`
  (set `self.Point Iterator` -1)
  (bind _returnvalue (`AddComponent|Static Mesh Component_8` :`RelativeTransform` (`KismetMathLibrary.MakeTransform` (0.0 0.0 0.0))))
  (`StaticMeshComponent.SetStaticMesh` _returnvalue "/Game/Shapes/Shape_Sphere.Shape_Sphere")
  (`self.Patrol To Next`))

(event `Patrol To Next`
  (bind _output_get (set `self.Point Iterator` (+ (`self.Point Iterator`) 1)))
  (`|AIMoveTo` "0" self (`self.K2_GetActorLocation` (`KismetArrayLibrary.Array_Get` (`self.Target Points`) _output_get))
    (:`then`
      (if (== _output_get (- (`KismetArrayLibrary.Array_Length` (`self.Target Points`)) 1))
        (set `self.Point Iterator` -1)))
    (:`OnSuccess`
      (`self.Patrol To Next` :!label _label))
    (:`OnFail`
      (goto _label))))

(fn `UserConstructionScript`)