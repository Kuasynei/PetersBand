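; Lever interactable that toggles its IsOn state and updates a linked WhatToAffect actor when tagged actors overlap it.
; An Anchovie overlap switches it off and an AntiChovie overlap switches it on, each playing its sound at the target.
; Target visibility and collision come from the overlapper's tags, so an actor with only one tag leaves the target visible and collidable in either direction.
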(event `self.ReceiveActorBeginOverlap`
  (params (OtherActor :type "Actor Object Reference"))
  (bind _returnvalue (`self.ActorHasTag` OtherActor "Anchovie"))
  (bind _returnvalue_2 (`self.ActorHasTag` OtherActor "AntiChovie"))
  (bind _whattoaffect (`self.WhatToAffect`))
  (bind _ison (`self.IsOn`))
  (bind _returnvalue_3 (`self.K2_GetActorLocation` _whattoaffect))
  (if _returnvalue
    (if _ison
      (`self.SetActorHiddenInGame` _whattoaffect _returnvalue_2)
      (`self.SetActorEnableCollision` _whattoaffect _returnvalue)
      (set `self.IsOn` false)
      (`GameplayStatics.PlaySoundAtLocation` (`self.ObjectDeactivationSound`) _returnvalue_3))
    (elif _returnvalue_2
      (if (not _ison)
        (`self.SetActorHiddenInGame` _whattoaffect _returnvalue)
        (`self.SetActorEnableCollision` _whattoaffect _returnvalue_2)
        (set `self.IsOn` true)
        (`GameplayStatics.PlaySoundAtLocation` (`self.ObjectActivationSound`) _returnvalue_3)))))

(fn `UserConstructionScript`)