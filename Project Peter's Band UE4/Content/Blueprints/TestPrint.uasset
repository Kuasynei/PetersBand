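; TestPrint is an actor that switches a runtime-added spot light component's activation based on the tags of actors that overlap it.
; On BeginPlay it adds the spot light, with a relative transform built from WhereToLight's negated up vector.
; An overlapping actor tagged "Anchovie" activates the component with reset, while one tagged "Antichovie" deactivates it.
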(event `self.ReceiveBeginPlay`
  (bind _returnvalue (`AddComponent|Spot Light Component_0` :`RelativeTransform` (`KismetMathLibrary.Conv_VectorToTransform` (* (`SceneComponent.GetUpVector` (`self.WhereToLight`)) -1)))))

(event `self.ReceiveActorBeginOverlap`
  (params (OtherActor :type "Actor Object Reference"))
  (bind _returnvalue (`self.ActorHasTag` OtherActor "Anchovie"))
  (if _returnvalue
    (`ActorComponent.Activate` (stale `self.ReceiveBeginPlay` _returnvalue) _returnvalue)
    (elif (`self.ActorHasTag` OtherActor "Antichovie")
      (`ActorComponent.Deactivate` (stale `self.ReceiveBeginPlay` _returnvalue)))))

(fn `UserConstructionScript`)